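; CCUBEE is an actor that moves back and forth along the Dir axis.
; Each Tick offsets its location by normalized Dir times Speed and delta time, without sweep, using the Stop boolean to pick forward or reverse.
; An accumulated timer flips Stop once it exceeds three seconds, then resets and prints the new value.
; Despite its name, Stop only selects direction and never halts movement.
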(event `self.ReceiveBeginPlay`)

(event `self.ReceiveTick`
  (params (DeltaSeconds :type "Float (single-precision)"))
  (`|ExecutionSequence`
    (:`then_0`
      (set `self.Acc time` (+ (`self.Acc time`) DeltaSeconds)))
    (:`then_1`
      (if (`self.stop`)
        (`self.K2_SetActorLocation` (+ (`self.K2_GetActorLocation`) (* (* (`KismetMathLibrary.Normal` (`self.Dir`)) (`self.speed`)) DeltaSeconds)))
        (else
          (`self.K2_SetActorLocation` (+ (`self.K2_GetActorLocation`) (* (* (`KismetMathLibrary.Normal` (* (`self.Dir`) -1.0)) (`self.speed`)) DeltaSeconds))))))
    (:`then_2`
      (if (> (`self.Acc time`) 3.0)
        (if (`self.stop`)
          (set `self.stop` false)
          (else
            (set `self.stop` true)))
        (set `self.Acc time` 0.0)
        (`KismetSystemLibrary.PrintString` (`KismetStringLibrary.Conv_BoolToString` (`self.stop`)))))))

(fn `UserConstructionScript`)