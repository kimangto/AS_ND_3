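; BP_InterectionActor is a timed interaction actor with a progress widget, tied to a monster supplied through SetMonster.
; While ONInterection is true, Tick accumulates time and passes the remaining fraction to the UI_Interection widget.
; At MaxTime it destroys both the monster and itself, provided the monster is valid.
; When ONInterection is false, it resets the timer and zeroes the widget component's Percent material parameter.
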(event `self.ReceiveTick`
  (params (DeltaSeconds :type "Float (single-precision)"))
  (bind _monsteractor (`self.MonsterActor`))
  (if (`self.ONInterection`)
    (set `self.AccTime` (+ (`self.AccTime`) DeltaSeconds))
    (bind _asui_interection (cast `/Game/01_Blueprints/04_UI/UI_Interection` (`WidgetComponent.GetWidget` (`self.Widget`))))
    (`/Game/01_Blueprints/04_UI/UI_Interection.SetPer` _asui_interection (- 1.0 (/ (`self.AccTime`) (`self.MaxTime`))))
    (if (>= (`self.AccTime`) (`self.MaxTime`))
      (`/Engine/EditorBlueprintResources/StandardMacros.IsValid` _monsteractor
        (:`Is Valid`
          (`self.K2_DestroyActor` _monsteractor)
          (`self.K2_DestroyActor`))))
    (else
      (set `self.AccTime` 0.0)
      (`MeshComponent.SetScalarParameterValueOnMaterials` (`self.Widget`) "Percent" 0.0))))

(event `SetMonster`
  (params (MonsterActor :type "Actor Object Reference"))
  (set `self.MonsterActor` MonsterActor))

(fn `UserConstructionScript`)