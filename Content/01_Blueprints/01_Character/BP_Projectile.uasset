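; Projectile actor that, on hit, sets off a field system and fire effects at the impact point.
; It spawns an FS_MasterField at the hit location, sets its activation type and triggers it, then calls AddMad on the player character and destroys itself shortly after.
; In parallel it activates its Niagara component and spawns a fire system, with a delayed deactivation that outlasts the actor's destroy delay.
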(event `self.ReceiveHit`
  (params (MyComp :type "PrimitiveComponent Object Reference") (Other :type "Actor Object Reference") (OtherComp :type "PrimitiveComponent Object Reference") (bSelfMoved :type Boolean) (HitLocation :type "Vector Structure") (HitNormal :type "Vector Structure") (NormalImpulse :type "Vector Structure") (Hit :type "HitResult Structure (by ref)"))
  (`|ExecutionSequence`
    (:`then_0`
      (bind _returnvalue (`|SpawnActorFromClass` "/Engine/EditorResources/FieldNodes/FS_MasterField.FS_MasterField_C" (`KismetMathLibrary.MakeTransform` HitLocation) "Undefined" "MultiplyWithRoot" null null))
      (set `/Engine/EditorResources/FieldNodes/FS_MasterField.ActivationType` "NewEnumerator4" _returnvalue)
      (`/Engine/EditorResources/FieldNodes/FS_MasterField.CE_Trigger` _returnvalue)
      (bind _asbp_base_character (cast `/Game/01_Blueprints/01_Character/BP_BaseCharacter` (`GameplayStatics.GetPlayerCharacter` 0)))
      (`/Game/01_Blueprints/01_Character/BP_BaseCharacter.AddMad` _asbp_base_character)
      (`KismetSystemLibrary.Delay` 0.2)
      (`self.K2_DestroyActor`))
    (:`then_1`
      (`ActorComponent.Activate` (`self.Niagara`) false)
      (`NiagaraFunctionLibrary.SpawnSystemAtLocation` "/Game/02_Resource/Niagara/NA_FireAnimation.NA_FireAnimation" HitLocation)
      (`KismetSystemLibrary.Delay` 1.0)
      (`ActorComponent.Deactivate` (`self.Niagara`)))))

(fn `UserConstructionScript`)