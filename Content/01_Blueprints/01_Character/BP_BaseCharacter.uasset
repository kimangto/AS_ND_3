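; Base player character Blueprint with Enhanced Input movement, jumping, mouse look, camera zoom and projectile shooting.
; BeginPlay adds the input mapping context, and movement follows control yaw only.
; The mouse wheel changes spring arm length without limits, as the clamp logic is disconnected.
; Left mouse Triggered calls Shootings, which spawns BP_Projectile ahead of the actor using its rotation rather than the camera's.
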(event `self.ReceiveBeginPlay`
  ;[1 1 1] enhanced input 설정
  (bind `_as플레이어_컨트롤러` (cast `PlayerController` (`self.GetController`)))
  (`/Engine/EditorBlueprintResources/StandardMacros.IsValid` `_as플레이어_컨트롤러`
    (:`Is Valid`
      (`EnhancedInputSubsystemInterface.AddMappingContext` (pcsubsystem `EnhancedInputLocalPlayerSubsystem` `_as플레이어_컨트롤러`) "/Game/01_Blueprints/00_Global/Infut/IM_Context.IM_Context" 0 (struct)))))

(event `self.ReceiveTick`
  (params (DeltaSeconds :type "Float (single-precision)")))

(event `EnhancedInput|/Game/01_Blueprints/00_Global/Infut/IA_Jump`
  (params (ActionValue :type Boolean) (ElapsedSeconds :type "Float (double-precision)") (TriggeredSeconds :type "Float (double-precision)") (InputAction :type "InputAction Object Reference" :default "/Game/01_Blueprints/00_Global/Infut/IA_Jump.IA_Jump"))
  ;[1 1 1] 점프 설정
  (:`Started`
    (`self.Jump`)))

(event `EnhancedInput|/Game/01_Blueprints/00_Global/Infut/IA_MoveFoward`
  (params (ActionValue :type "Float (double-precision)") (ElapsedSeconds :type "Float (double-precision)") (TriggeredSeconds :type "Float (double-precision)") (InputAction :type "InputAction Object Reference" :default "/Game/01_Blueprints/00_Global/Infut/IA_MoveFoward.IA_MoveFoward"))
  (bind (_returnvalue_roll _returnvalue_pitch _returnvalue_yaw) (`KismetMathLibrary.BreakRotator` (`self.GetControlRotation`)))
  ;[1 1 1] 앞뒤로 움직이기
  (:`Triggered`
    (`self.AddMovementInput` (`KismetMathLibrary.GetForwardVector` (`KismetMathLibrary.MakeRotator` 0.0 0.0 _returnvalue_yaw)) ActionValue)))

(event `EnhancedInput|/Game/01_Blueprints/00_Global/Infut/IA_MoveRight`
  (params (ActionValue :type "Float (double-precision)") (ElapsedSeconds :type "Float (double-precision)") (TriggeredSeconds :type "Float (double-precision)") (InputAction :type "InputAction Object Reference" :default "/Game/01_Blueprints/00_Global/Infut/IA_MoveRight.IA_MoveRight"))
  (bind (_returnvalue_roll _returnvalue_pitch _returnvalue_yaw) (`KismetMathLibrary.BreakRotator` (`self.GetControlRotation`)))
  ;[1 1 1] 옆으로 움직이기
  (:`Triggered`
    (`self.AddMovementInput` (`KismetMathLibrary.GetRightVector` (`KismetMathLibrary.MakeRotator` 0.0 0.0 _returnvalue_yaw)) ActionValue)))

(event `EnhancedInput|/Game/01_Blueprints/00_Global/Infut/IA_MouseXY`
  (params (ActionValue :type "Vector2D Structure") (ElapsedSeconds :type "Float (double-precision)") (TriggeredSeconds :type "Float (double-precision)") (InputAction :type "InputAction Object Reference" :default "/Game/01_Blueprints/00_Global/Infut/IA_MouseXY.IA_MouseXY"))
  ;[1 1 1] 마우스로 화면 돌리기
  (:`Triggered`
    (`self.AddControllerYawInput` ActionValue_X)
    (`self.AddControllerPitchInput` ActionValue_Y)))

(event `EnhancedInput|/Game/01_Blueprints/00_Global/Infut/IA_Mousejoominout`
  (params (ActionValue :type "Float (double-precision)") (ElapsedSeconds :type "Float (double-precision)") (TriggeredSeconds :type "Float (double-precision)") (InputAction :type "InputAction Object Reference" :default "/Game/01_Blueprints/00_Global/Infut/IA_Mousejoominout.IA_Mousejoominout"))
  ;[1 1 1] 마우스 휠 줌아웃
  (:`Triggered`
    (set `SpringArmComponent.TargetArmLength` (+ (`SpringArmComponent.TargetArmLength` (`self.SpringArm`)) (* (`self.TargetArmLength`) ActionValue)) (`self.SpringArm`))))

(event `EnhancedInput|/Game/01_Blueprints/00_Global/Infut/IA_MouseLeft`
  (params (ActionValue :type Boolean) (ElapsedSeconds :type "Float (double-precision)") (TriggeredSeconds :type "Float (double-precision)") (InputAction :type "InputAction Object Reference" :default "/Game/01_Blueprints/00_Global/Infut/IA_MouseLeft.IA_MouseLeft"))
  (:`Triggered`
    (`self.Shootings`)))

(fn `Shootings`
  (bind (_returnvalue_location _returnvalue_rotation _returnvalue_scale) (`KismetMathLibrary.BreakTransform` (`self.GetTransform`)))
  (`|SpawnActorFromClass` "/Game/01_Blueprints/01_Character/BP_Projectile.BP_Projectile_C" (`KismetMathLibrary.MakeTransform` (+ _returnvalue_location (* (`self.GetActorForwardVector`) 150.0)) _returnvalue_rotation _returnvalue_scale) "Undefined" "MultiplyWithRoot" null null))

(fn `UserConstructionScript`)