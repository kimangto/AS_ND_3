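; BP_MainHUD is the main HUD Blueprint, which puts the game's main and settings widgets on screen.
; On BeginPlay it creates UI_Main for the first player controller, adds it to the viewport and stores the reference.
; The ShowSetingUI event creates, displays and focuses UI_Setting when no valid instance exists; otherwise it only makes the cached widget visible, without refocusing it.
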(event `self.ReceiveBeginPlay`
  (bind _returnvalue (`|CreateWidget` "/Game/01_Blueprints/04_UI/UI_Main.UI_Main_C" (`GameplayStatics.GetPlayerController` 0)))
  ;[1 1 1] ui를 보여줄거야 - zorder 높을수록 위에보임
  (`UserWidget.AddToViewport` _returnvalue 0)
  (set `self.MainUI` _returnvalue))

(event `ShowSetingUI`
  (bind _settinui (`self.SettinUI`))
  (`/Engine/EditorBlueprintResources/StandardMacros.IsValid` _settinui
    (:`Is Valid`
      (`Widget.SetVisibility` _settinui "Visible"))
    (:`Is Not Valid`
      (bind _returnvalue (`|CreateWidget` "/Game/01_Blueprints/04_UI/UI_Setting.UI_Setting_C"))
      (bind _output_get (set `self.SettinUI` _returnvalue))
      (`UserWidget.AddToViewport` _output_get 0)
      (`Widget.SetFocus` (`self.SettinUI`)))))

(fn `UserConstructionScript`)